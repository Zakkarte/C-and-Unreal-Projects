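; BP_Maze is a tiltable maze board that the player rotates with the TiltForward and TiltRight axis inputs.
; Each input adds rotation scaled by RotationSpeed, then clamps that axis to a small symmetric range around level.
; Forward tilt works on world-space pitch, while right tilt works on local roll.
; GetGoal exposes the Goal child actor cast to BP_Goal.
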(event `InputAxis|TiltForward`
  (params (AxisValue :type "Float (single-precision)"))
  (bind (_returnvalue_roll _returnvalue_pitch _returnvalue_yaw) (`KismetMathLibrary.BreakRotator` (`SceneComponent.K2_GetComponentRotation` (`self.BoardMesh`))))
  (`SceneComponent.K2_AddWorldRotation` (`self.BoardMesh`) (`KismetMathLibrary.MakeRotator` 0.0 (* AxisValue (`self.RotationSpeed`))) false false)
  (`SceneComponent.K2_SetWorldRotation` (`self.BoardMesh`) (`KismetMathLibrary.MakeRotator` _returnvalue_roll (`KismetMathLibrary.FClamp` _returnvalue_pitch -5.0 5.0) _returnvalue_yaw) false false))

(event `InputAxis|TiltRight`
  (params (AxisValue :type "Float (single-precision)"))
  (bind (_relativerotation_roll _relativerotation_pitch _relativerotation_yaw) (`KismetMathLibrary.BreakRotator` (`SceneComponent.RelativeRotation` (`self.BoardMesh`))))
  (`SceneComponent.K2_AddLocalRotation` (`self.BoardMesh`) (`KismetMathLibrary.MakeRotator` (* AxisValue (`self.RotationSpeed`))) false false)
  (`SceneComponent.K2_SetRelativeRotation` (`self.BoardMesh`) (`KismetMathLibrary.MakeRotator` (`KismetMathLibrary.FClamp` _relativerotation_roll -5.0 5.0) _relativerotation_pitch _relativerotation_yaw) false false))

(fn `GetGoal`
  (returns (`AsBP Goal` :type "/Game/BP_Goal Object Reference"))
  (return (cast `/Game/BP_Goal` (`ChildActorComponent.ChildActor` (`self.Goal`)) :!pure true)))

(fn `UserConstructionScript`)