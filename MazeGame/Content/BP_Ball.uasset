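; BP_Ball is a physics ball for a maze game that returns to its start point when it reaches the goal or falls out.
; BeginPlay stores the starting location and binds to the overlap dispatcher on the Maze's goal.
; Tick checks whether the ball has dropped below KillHeight.
; Both triggers call ResetBall, which moves the actor back and zeroes the mesh's linear velocity.
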(event `self.ReceiveBeginPlay`
  (set `self.StartingLocation` (`self.K2_GetActorLocation`))
  (add `/Game/BP_Goal.OnBallOverLap` (`/Game/BP_Maze.GetGoal` (`self.Maze`)) (delegate `OnBallOverLap_Event_0`)))

(event `OnBallOverLap_Event_0`
  (`self.ResetBall`))

(event `self.ReceiveTick`
  (params (DeltaSeconds :type "Float (single-precision)"))
  (bind (_returnvalue_x _returnvalue_y _returnvalue_z) (`KismetMathLibrary.BreakVector` (`self.K2_GetActorLocation`)))
  (if (< _returnvalue_z (`self.KillHeight`))
    (`self.ResetBall`)))

(fn `ResetBall`
  (`self.K2_SetActorLocation` (`self.StartingLocation`))
  (`PrimitiveComponent.SetPhysicsLinearVelocity` (`self.BallMesh`) (0.0 0.0 0.0) false "None"))

(fn `UserConstructionScript`)